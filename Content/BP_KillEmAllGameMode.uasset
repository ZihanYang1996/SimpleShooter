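; BP_KillEmAllGameMode is a game mode Blueprint that controls which screen-level UI widget the player sees.
; SetupHUD creates the shooter character HUD and stores it as the current viewport widget.
; DisplayLoseScreen and DisplayWinScreen remove that widget and replace it with the lose or win screen.
; It holds no match rules; these events are not called within this graph, and BeginPlay and Tick are unused.
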(event `self.SetupHUD`
  (bind _returnvalue (`|CreateWidget` "/Game/Character/WB_ShooterCharacter.WB_ShooterCharacter_C"))
  (bind _output_get (set `self.CurrentWidgetOnViewport` _returnvalue))
  (`UserWidget.AddToViewport` _output_get 0))

(event `self.DisplayLoseScreen`
  (`Widget.RemoveFromParent` (`self.CurrentWidgetOnViewport`))
  (bind _returnvalue (`|CreateWidget` "/Game/WB_LoseScreen.WB_LoseScreen_C"))
  (bind _output_get (set `self.CurrentWidgetOnViewport` _returnvalue))
  (`UserWidget.AddToViewport` _output_get 0))

(event `self.DisplayWinScreen`
  (`Widget.RemoveFromParent` (`self.CurrentWidgetOnViewport`))
  (bind _returnvalue (`|CreateWidget` "/Game/WB_WinScreen.WB_WinScreen_C"))
  (bind _output_get (set `self.CurrentWidgetOnViewport` _returnvalue))
  (`UserWidget.AddToViewport` _output_get 0))

(fn `UserConstructionScript`)